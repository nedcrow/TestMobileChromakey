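; BP_SelfiePawn is a remote virtual camera test pawn that drives a Python "selfie" script, with mouse-look and axis movement.
; BeginPlay shows the cursor, imports the selfie module through ExecutePythonScript and calls CanURL on a hard-coded LAN snapshot URL.
; While CanURL is true, Tick runs the script's selfie() every frame and, if UseDEVICE is set, copies tracked device 0's pose onto the pawn.
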(event EventBeginPlay
  (Variables|/Script/Engine.PlayerController|SetbShowMouseCursor (Game|GetPlayerController 0) true)
  ;[1 1 1] Import selfie script
  (Class|CppLib|ExecutePythonScript "import selfie as s 
from importlib import * 
reload(s)")
  (Class|CppLib|CanURL "http://192.168.1.215:8080/shot.jpg"))

(event EventTick
  (params (DeltaSeconds :type Float%20%28single-precision%29))
  (bind (_outposition _outorientation) (Class|SteamVRFunctionLibrary|GetTrackedDevicePositionandOrientation))
  (if (Variables|Default|GetbCanURL)
    (Class|CppLib|ExecutePythonScript "s.selfie()")
    ;[1 1 1] Movement from device
    (if (Variables|Default|GetuseDEVICE)
      (Transformation|SetActorRelativeTransform (Math|Transform|MakeTransform _outposition _outorientation) false false))))

(event Input|AxisEvents|InputAxisForward
  (params (AxisValue :type Float%20%28single-precision%29))
  (Pawn|Input|AddMovementInput (Math|Vector|GetForwardVector (Pawn|GetControlRotation :!class /Script/Engine.Pawn)) (* AxisValue (Variables|Default|GetMoveSpeed)) false))

(event Input|AxisEvents|InputAxisRight
  (params (AxisValue :type Float%20%28single-precision%29))
  (Pawn|Input|AddMovementInput (Math|Vector|GetRightVector (Pawn|GetControlRotation :!class /Script/Engine.Pawn)) (* AxisValue (Variables|Default|GetMoveSpeed)) false))

(event Input|MouseEvents|Mouse2D
  (params (AxisValue :type Vector :default "0, 0, 0"))
  (bind _returnvalue (Game|GetPlayerController 0))
  (Class|PlayerController|AddYawInput _returnvalue (.x AxisValue))
  (Class|PlayerController|AddPitchInput _returnvalue (* (.y AxisValue) -1.0)))

(fn ConstructionScript)

(fn CallSelfiefromPythonScript
  (Class|CppLib|ExecutePythonScript "s.selfie()"))