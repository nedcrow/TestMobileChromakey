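; Remote-camera test pawn that puts the MainWidget_RC UI on screen at BeginPlay, after calling TestMessageFunction.
; SetTextureFromWebCamWidget feeds the render target of WidgetComp into the Color parameter of the dynamic material on the main widget's Image0, mirroring one widget inside another.
; It prints an error when Image0 is invalid and is not called within this graph.
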(event EventBeginPlay
  (Class|MobileHelperBPLibrary|TestMessageFunction)
  (bind _returnvalue (UserInterface|CreateWidget "/Game/TestRemoteVCam/Blueprints/MainWidget_RC.MainWidget_RC_C"))
  (bind _output_get (Variables|Default|SetMaindget _returnvalue))
  (UserInterface|Viewport|AddtoViewport _output_get 0))

(event Collision|EventActorBeginOverlap
  (params (OtherActor :type Actor%20Object%20Reference)))

(event EventTick
  (params (DeltaSeconds :type Float%20%28single-precision%29)))

(fn ConstructionScript)

(fn SetTexturefromWebCamWidget
  (bind _maindget (Variables|Default|GetMaindget))
  (bind _image_0 (Variables|/Game/TestRemoteVCam/Blueprints/MainWidget_RC.MainWidget_RC_C|GetImage_0 _maindget))
  (if (Utilities|IsValid _image_0)
    (bind _returnvalue (Appearance|GetDynamicMaterial _image_0 :!class /Script/UMG.Image))
    (Rendering|Material|SetTextureParameterValue _returnvalue "Color" (Class|WidgetComponent|GetRenderTarget (Variables|Default|GetWidgetComp)))
    (else
      (Development|PrintString "Null MIDynamic"))))