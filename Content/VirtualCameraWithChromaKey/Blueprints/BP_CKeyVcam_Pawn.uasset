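; Virtual camera pawn that rotates the view through either touch drags or device motion.
; The first finger's drag drives yaw and pitch, and the second finger's horizontal offset drives roll.
; ChangeRotateMode switches between touch input and a looping Co_RotationRate timer that applies gyro rotation rates, flipping roll direction by tilt, with input disabled.
; AR session start, geometry debug drawing and status printing are present but never run.
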(event EventBeginPlay)

(event Input|TouchEvents|InputTouch
  (params (Location :type Vector) (FingerIndex :type ETouchIndex%20Enum))
  (bind _returnvalue (Game|Player|GetPlayerPawn 0))
  (bind _speed_yawpitch (Variables|Default|GetSpeed_YawPitch))
  (:Pressed
    ;[1 1 1] Setup Move
    (switch Utilities|FlowControl|Switch|SwitchonETouchIndex FingerIndex
      (:Touch1
        (Variables|Default|SetLocationTouchStart Location))
      (:Touch2
        (if (not (Variables|Default|GetPressing))
          (Variables|Default|SetLocationTouchEnd Location)
          (Variables|Default|SetPressing true)))))
  (:Released
    (switch Utilities|FlowControl|Switch|SwitchonETouchIndex FingerIndex
      (:Touch2
        (Variables|Default|SetPressing false))))
  (:Moved
    (switch Utilities|FlowControl|Switch|SwitchonETouchIndex FingerIndex
      (:Touch1
        ;[1 1 1] Rotation
        (Pawn|Input|AddControllerYawInput _returnvalue (* (.X (Math|Vector|BreakVector (- (Variables|Default|GetLocationTouchStart) Location))) (* _speed_yawpitch 1.0)))
        (Pawn|Input|AddControllerPitchInput _returnvalue (* (.Y (Math|Vector|BreakVector (- (Variables|Default|GetLocationTouchStart) Location))) (* 1.0 _speed_yawpitch)))
        (Variables|Default|SetLocationTouchStart Location))
      (:Touch2
        (Pawn|Input|AddControllerRollInput (Game|Player|GetPlayerPawn 0) (* (.X (Math|Vector|BreakVector (- (Variables|Default|GetLocationTouchEnd) Location))) (Variables|Default|GetSpeed_Roll)))))))

(fn ConstructionScript)

(fn CoRotationRate
  (bind _returnvalue (Game|GetPlayerController 0))
  (bind (_tilt _rotationrate) (Class|PlayerController|GetInputMotionState _returnvalue))
  (bind _returnvalue_2 (* (.z _rotationrate) -1.96))
  (Pawn|Input|AddControllerPitchInput (* (.y _rotationrate) 1.0))
  (Pawn|Input|AddControllerYawInput (* (.x _rotationrate) 11.0))
  (if (< (.y _tilt) 0.0)
    (Pawn|Input|AddControllerRollInput _returnvalue_2)
    (else
      (Pawn|Input|AddControllerRollInput (* _returnvalue_2 -1.0)))))

(fn ChangeRotateMode
  (params (NewParam :type E_RotateMode%20Enum :default "NewEnumerator0"))
  (bind _returnvalue (Game|GetPlayerController 0))
  (Utilities|Time|ClearTimerbyFunctionName 0 "Co_RotationRate")
  (switch Utilities|FlowControl|Switch|SwitchonE_RotateMode NewParam
    (:NewEnumerator0
      (Utilities|Time|ClearTimerbyFunctionName 0 "Co_RotationRate")
      (Input|EnableInput _returnvalue))
    (:NewEnumerator1
      (Utilities|Time|SetTimerbyFunctionName 0 "Co_RotationRate" (Variables|Default|GetLoopingSecond) true)
      (Input|DisableInput _returnvalue))))