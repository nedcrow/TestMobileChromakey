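; Virtual camera pawn that looks and moves through touch input or the device's motion sensors.
; The first finger drags yaw and pitch, while the second drives movement along the control rotation's forward and right vectors.
; ChangeRotateMode either enables touch input or disables it and loops a timer applying gyro rotation rate, with tilt-dependent roll sign.
; A smoothed tilt-to-rotation function exists, but this file never starts it.
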(event EventBeginPlay)

(event EventTick
  (params (DeltaSeconds :type Float%20%28single-precision%29)))

(event Input|TouchEvents|InputTouch
  (params (Location :type Vector) (FingerIndex :type ETouchIndex%20Enum))
  (bind _returnvalue (Game|Player|GetPlayerPawn 0))
  (bind _returnvalue_2 (Game|Player|GetPlayerPawn 0))
  (bind _rotatespeed (Variables|Default|GetRotateSpeed))
  (bind _rotatespeed_2 (Variables|Default|GetRotateSpeed))
  (bind _returnvalue_3 (Pawn|GetControlRotation _returnvalue_2 :!class /Script/Engine.Pawn))
  (:Pressed
    ;[1 1 1] Setup Move
    (switch Utilities|FlowControl|Switch|SwitchonETouchIndex FingerIndex
      (:Touch1
        (Variables|Default|SetLocationTouchStart Location))
      (:Touch2
        (if (not (Variables|Default|GetPressing))
          (Variables|Default|SetLocationTouchEnd Location)
          (Variables|Default|SetPressing true)))))
  (:Released
    (switch Utilities|FlowControl|Switch|SwitchonETouchIndex FingerIndex
      (:Touch2
        (Variables|Default|SetPressing false))))
  (:Moved
    (switch Utilities|FlowControl|Switch|SwitchonETouchIndex FingerIndex
      (:Touch1
        ;[1 1 1] Rotation
        (Pawn|Input|AddControllerYawInput _returnvalue (* (.X (Math|Vector|BreakVector (- (Variables|Default|GetLocationTouchStart) Location))) (* _rotatespeed_2 -1.0)))
        (Pawn|Input|AddControllerPitchInput _returnvalue (* (.Y (Math|Vector|BreakVector (- (Variables|Default|GetLocationTouchStart) Location))) (* 1.0 _rotatespeed_2)))
        (Variables|Default|SetLocationTouchStart Location))
      (:Touch2
        ;[1 1 1] Movement
        (Pawn|Input|AddMovementInput _returnvalue_2 (Math|Vector|GetRightVector _returnvalue_3) (* (.X (Math|Vector|BreakVector (- (Variables|Default|GetLocationTouchEnd) Location))) _rotatespeed) false)
        (Pawn|Input|AddMovementInput _returnvalue_2 (Math|Vector|GetForwardVector _returnvalue_3) (* (.Y (Math|Vector|BreakVector (- (Variables|Default|GetLocationTouchEnd) Location))) _rotatespeed) false)))))

(fn ConstructionScript)

(fn CoRotationRate
  (bind _returnvalue (Game|GetPlayerController 0))
  (bind (_tilt _rotationrate) (Class|PlayerController|GetInputMotionState _returnvalue))
  (bind _returnvalue_2 (* (.z _rotationrate) -1.96))
  (Pawn|Input|AddControllerPitchInput (* (.y _rotationrate) -1.0))
  (Pawn|Input|AddControllerYawInput (* (.x _rotationrate) 1.0))
  (if (< (.y _tilt) 0.0)
    (Pawn|Input|AddControllerRollInput _returnvalue_2)
    (Development|PrintString "True")
    (else
      (Pawn|Input|AddControllerRollInput (* _returnvalue_2 -1.0))
      (Development|PrintString "False"))))

(fn CoRotationTilt
  (bind _output_get (Variables|Default|SetTempTilt (.Tilt (Class|PlayerController|GetInputMotionState (Game|GetPlayerController 0)))))
  (Variables|Default|SetCurrentTilt _output_get)
  (Variables|Default|SetTiltDist (Math|Vector|Distance(Vector) (Variables|Default|GetLastTilt) (Variables|Default|GetTempTilt)))
  (if (< (Variables|Default|GetTiltDist) 0.4)
    (Variables|Default|SetCurrentTilt (Math|Vector|Lerp(Vector) (Variables|Default|GetLastTilt) (Variables|Default|GetCurrentTilt) (/ (Variables|Default|GetTiltDist) 6.28)))
    (elif (< (Variables|Default|GetTiltDist) 2.0)
      (Variables|Default|SetCurrentTilt (Math|Vector|Lerp(Vector) (Variables|Default|GetLastTilt) (Variables|Default|GetCurrentTilt) (* (/ (Variables|Default|GetTiltDist) 6.28) 0.01)))
      (else
        (if (< (Variables|Default|GetTiltDist) 3.14)
          (Variables|Default|SetCurrentTilt (Math|Vector|MakeVector (.x (Variables|Default|GetCurrentTilt)) (.y (Variables|Default|GetCurrentTilt)) (- (Variables|Default|GetTiltDist) 6.24)))
          (else
            (Variables|Default|SetCurrentTilt (Math|Vector|MakeVector (.x (Variables|Default|GetCurrentTilt)) (.y (Variables|Default|GetCurrentTilt)) (Variables|Default|GetTiltDist)))))
        ;[1 1 1] 코멘트
        (Variables|Default|SetCurrentTilt (Math|Vector|Lerp(Vector) (Variables|Default|GetLastTilt) (Variables|Default|GetCurrentTilt) 0.01)))))
  (Pawn|SetControlRotation (Game|GetPlayerController 0) (Math|Conversions|RotationFromXVector (Math|Rotator|GetRotationXVector (Math|Rotator|MakeRotator (Math|Trig|RadiansToDegrees (.x (Variables|Default|GetCurrentTilt))) (+ (Math|Trig|RadiansToDegrees (.y (Variables|Default|GetCurrentTilt))) -9e+01) (Math|Trig|RadiansToDegrees (.z (Variables|Default|GetCurrentTilt)))))))
  (Variables|Default|SetLastTilt (Variables|Default|GetCurrentTilt))
  (Development|PrintString (Utilities|String|Append (Utilities|String|Append (Utilities|String|ToString(Float) (Variables|Default|GetTiltDist)) "_____") (Utilities|String|ToString(Vector) (Variables|Default|GetLastTilt)))))

(fn ChangeRotateMode
  (params (NewParam :type E_RotateMode%20Enum :default "NewEnumerator0"))
  (bind _returnvalue (Game|Player|GetPlayerPawn 0))
  (Utilities|Time|ClearTimerbyFunctionName 0 "Co_RotationTilt")
  (Utilities|Time|ClearTimerbyFunctionName 0 "Co_RotationRate")
  (switch Utilities|FlowControl|Switch|SwitchonE_RotateMode NewParam
    (:NewEnumerator0
      (Utilities|Time|ClearTimerbyFunctionName 0 "Co_RotationRate")
      (Input|EnableInput _returnvalue 0))
    (:NewEnumerator1
      (Utilities|Time|SetTimerbyFunctionName 0 "Co_RotationRate" (Variables|Default|GetLoopingSecond_RR) true)
      (Input|DisableInput _returnvalue 0))))